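; Blueprint library that records per-chapter progress, including connection points and completed minigames, in the save game.
; Both functions fetch the current chapter's statistics from BP_SaveGame through the VN save and chapter subsystems, then write back an updated end-game stat struct.
; AddConnectionPoints adds a delta to the chapter score.
; NotifyMinigameComplete, only on success, increments the completed minigame count and adds the awarded points.
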(fn `Add Connection Points`
  (params (`Delta Points` :type Integer))
  (bind _asbp_save_game (cast `/Game/Game/Blueprints/BP_SaveGame` (`VNSaveSubsystem.SaveGame` (subsystem `VNSaveSubsystem`))))
  (bind (_minigamescompleted _score _customattribs) (break `/Game/Game/Blueprints/EndGame/ST_EndGameStat` (`/Game/Game/Blueprints/BP_SaveGame.Get Chapter Statistics` _asbp_save_game (`VNChapterSubsystem.CurrentChapterName` (subsystem `VNChapterSubsystem`)))))
  (`/Game/Game/Blueprints/BP_SaveGame.Update Chapter Statistics` _asbp_save_game (`VNChapterSubsystem.CurrentChapterName` (subsystem `VNChapterSubsystem`)) (make `/Game/Game/Blueprints/EndGame/ST_EndGameStat` _minigamescompleted (+ _score `Delta Points`) _customattribs)))

(fn `Notify Minigame Complete`
  (params (Success :type Boolean) (`Connection Points` :type Integer))
  (bind _currentchaptername (`VNChapterSubsystem.CurrentChapterName` (subsystem `VNChapterSubsystem`)))
  (bind _asbp_save_game (cast `/Game/Game/Blueprints/BP_SaveGame` (`VNSaveSubsystem.SaveGame` (subsystem `VNSaveSubsystem`))))
  (if Success
    (bind (_minigamescompleted _score _customattribs) (break `/Game/Game/Blueprints/EndGame/ST_EndGameStat` (`/Game/Game/Blueprints/BP_SaveGame.Get Chapter Statistics` _asbp_save_game _currentchaptername)))
    (`/Game/Game/Blueprints/BP_SaveGame.Update Chapter Statistics` _asbp_save_game _currentchaptername (make `/Game/Game/Blueprints/EndGame/ST_EndGameStat` (+ _minigamescompleted 1) (+ _score `Connection Points`) _customattribs))))