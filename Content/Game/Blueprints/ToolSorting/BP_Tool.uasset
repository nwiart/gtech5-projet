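; BP_Tool is a tool actor, apparently for a tool-sorting task, that the player picks up and drops with mouse clicks.
; Clicking its Cube toggles selection; while selected, Tick moves the Cube to the cursor's Visibility trace XY at a held height.
; Dropping restores a rest height cached at BeginPlay from the truncated starting Z plus an offset.
; The world-space hit point is applied directly as the Cube's relative location.
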(event `self.ReceiveBeginPlay`
  (bind (_relativelocation_x _relativelocation_y _relativelocation_z) (`KismetMathLibrary.BreakVector` (`SceneComponent.RelativeLocation` (`self.Cube`))))
  (set `self.ObjectRestHeight` (`KismetMathLibrary.Conv_IntToDouble` (+ (`KismetMathLibrary.FTrunc` _relativelocation_z) 10))))

(event `self.Cube.OnClicked`
  (params (TouchedComponent :type "PrimitiveComponent Object Reference") (ButtonPressed :type "Key Structure"))
  (bind _cube (`self.Cube`))
  (bind (_relativelocation_x _relativelocation_y) (`KismetMathLibrary.BreakVector` (`SceneComponent.RelativeLocation` _cube)))
  (if (`self.IsSelected`)
    (set `self.IsSelected` false)
    (`SceneComponent.K2_SetRelativeLocation` _cube (`KismetMathLibrary.MakeVector` _relativelocation_x _relativelocation_y (`self.ObjectRestHeight`)) false true)
    (else
      (set `self.IsSelected` true))))

(event `self.ReceiveTick`
  (params (DeltaSeconds :type "Float (single-precision)"))
  (bind (_x _y) (`KismetMathLibrary.BreakVector2D` (`KismetMathLibrary.Conv_VectorToVector2D` (`.Location` (`GameplayStatics.BreakHitResult` (`PlayerController.GetHitResultUnderCursorByChannel` (`GameplayStatics.GetPlayerController` 0) "TraceTypeQuery1" false))))))
  (if (`self.IsSelected`)
    (`SceneComponent.K2_SetRelativeLocation` (`self.Cube`) (`KismetMathLibrary.MakeVector` _x _y (`self.ObjectHeldHeight`)) false true)))

(fn `UserConstructionScript`)