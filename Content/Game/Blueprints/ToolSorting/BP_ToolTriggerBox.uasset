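; BP_ToolTriggerBox is a drop zone in the tool sorting minigame that detects when its matching tool sits inside it.
; On begin and end overlap, it compares the BP_Tool's ToolIndex to its ToolTriggerIndex and sets or clears TriggerValidated.
; It then adds or removes that tool as validated on the BP_ToolSortingManager, obtained from the VN chapter subsystem's MinigameManager.
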(event `self.TriggerBox.OnComponentBeginOverlap`
  (params (OverlappedComponent :type "PrimitiveComponent Object Reference") (OtherActor :type "Actor Object Reference") (OtherComp :type "PrimitiveComponent Object Reference") (OtherBodyIndex :type Integer) (bFromSweep :type Boolean) (SweepResult :type "HitResult Structure (by ref)"))
  (bind _asbp_tool (cast `/Game/Game/Blueprints/ToolSorting/BP_Tool` OtherActor))
  (if (== (`/Game/Game/Blueprints/ToolSorting/BP_Tool.ToolIndex` _asbp_tool) (`self.ToolTriggerIndex`))
    (set `self.TriggerValidated` true)
    (bind _asbp_tool_sorting_game_mode (cast `/Game/Game/Blueprints/ToolSorting/BP_ToolSortingManager` (`VNChapterSubsystem.MinigameManager` (subsystem `VNChapterSubsystem`))))
    (`/Game/Game/Blueprints/ToolSorting/BP_ToolSortingManager.AddValidatedTool` _asbp_tool_sorting_game_mode _asbp_tool)))

(event `self.TriggerBox.OnComponentEndOverlap`
  (params (OverlappedComponent :type "PrimitiveComponent Object Reference") (OtherActor :type "Actor Object Reference") (OtherComp :type "PrimitiveComponent Object Reference") (OtherBodyIndex :type Integer))
  (bind _asbp_tool (cast `/Game/Game/Blueprints/ToolSorting/BP_Tool` OtherActor))
  (if (== (`/Game/Game/Blueprints/ToolSorting/BP_Tool.ToolIndex` _asbp_tool) (`self.ToolTriggerIndex`))
    (set `self.TriggerValidated` false)
    (bind _asbp_tool_sorting_game_mode (cast `/Game/Game/Blueprints/ToolSorting/BP_ToolSortingManager` (`VNChapterSubsystem.MinigameManager` (subsystem `VNChapterSubsystem`))))
    (`/Game/Game/Blueprints/ToolSorting/BP_ToolSortingManager.RemoveValidatedTool` _asbp_tool_sorting_game_mode _asbp_tool)))

(fn `UserConstructionScript`)