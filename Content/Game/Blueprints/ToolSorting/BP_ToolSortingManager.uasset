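; BP_ToolSortingManager runs the tool sorting minigame and decides when it is won.
; It keeps a count of validated tools, raised and lowered by add and remove events.
; When the count matches the total, it completes the minigame as a success and deselects the last tool.
; It builds the minigame result with a fixed connection score delta and a hard-coded "Pass" stat for sorting every object.
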(event `AddValidatedTool`
  (params (Tool :type "/Game/Game/Blueprints/ToolSorting/BP_Tool Object Reference"))
  (bind _output_get (set `self.NumberOfValidatedTools` (+ (`self.NumberOfValidatedTools`) 1)))
  (if (== _output_get (`self.NumberOfTools`))
    (`self.OnMinigameComplete` true)
    (set `/Game/Game/Blueprints/ToolSorting/BP_Tool.IsSelected` false Tool)))

(event `RemoveValidatedTool`
  (params (Tool :type "/Game/Game/Blueprints/ToolSorting/BP_Tool Object Reference"))
  (set `self.NumberOfValidatedTools` (- (`self.NumberOfValidatedTools`) 1)))

(fn `BuildMinigameResult`
  (params (bSuccess :type Boolean))
  (returns (ReturnValue :type "MinigameResult Structure"))
  (return (make `MinigameResult` bSuccess 10 "Tool Sorting Game" (`|MakeMap` "Trier tous les objets dans le bon emplacement" "Pass" :!valuetype "Text"))))

(fn `UserConstructionScript`)