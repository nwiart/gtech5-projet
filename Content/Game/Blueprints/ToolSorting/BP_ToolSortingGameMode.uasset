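; BP_ToolSortingGameMode is the game mode for the Tool Sorting minigame, tracking how many tools are validated.
; Add and remove events adjust a validated-tool counter, and reaching the total tool count completes the minigame as a success.
; BuildMinigameResult packages the success flag with a fixed connection score delta, the game name and a custom stat that always reads Pass.
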(event `AddValidatedTool`
  (bind _output_get (set `self.NumberOfValidatedTools` (+ (`self.NumberOfValidatedTools`) 1)))
  (if (== _output_get (`self.NumberOfTools`))
    (`self.OnMinigameComplete` true)))

(event `RemoveValidatedTool`
  (set `self.NumberOfValidatedTools` (- (`self.NumberOfValidatedTools`) 1)))

(fn `BuildMinigameResult`
  (params (bSuccess :type Boolean))
  (returns (ReturnValue :type "MinigameResult Structure"))
  (return (make `MinigameResult` bSuccess 10 "Tool Sorting Game" (`|MakeMap` "Sorting all the items to the right position" "Pass" :!valuetype "Text"))))

(fn `UserConstructionScript`)