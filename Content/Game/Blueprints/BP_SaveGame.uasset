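; Save game object that stores end-game statistics for each chapter, tracking minigames completed and score.
; Statistics live in a map keyed by chapter name.
; The getter returns the stored entry, or adds and returns a zeroed one when the chapter is missing.
; The update function writes the given statistics into the map, replacing any existing entry for that chapter.
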(fn `Get Chapter Statistics`
  (params (`Chapter Name` :type Name))
  (returns (Stats :type "/Game/Game/Blueprints/EndGame/ST_EndGameStat Structure"))
  (bind _st_endgamestat (make `/Game/Game/Blueprints/EndGame/ST_EndGameStat` 0))
  (bind (_value _returnvalue) (`BlueprintMapLibrary.Map_Find` (`self.Chapter Statistics`) `Chapter Name`))
  (if _returnvalue
    (return _value)
    (else
      (`BlueprintMapLibrary.Map_Add` (`self.Chapter Statistics`) `Chapter Name` _st_endgamestat)
      (return _st_endgamestat))))

(fn `Update Chapter Statistics`
  (params (`Chapter Name` :type Name) (Statistics :type "/Game/Game/Blueprints/EndGame/ST_EndGameStat Structure"))
  (`BlueprintMapLibrary.Map_Add` (`self.Chapter Statistics`) `Chapter Name` Statistics))