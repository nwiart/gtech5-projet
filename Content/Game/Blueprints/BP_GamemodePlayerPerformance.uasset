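; Game mode for point-and-click, viewpoint-based play that shows the mouse cursor and a performance bar widget on start.
; TravelTo fades the HUD, teleports the player pawn to the target point of view's eye location and updates the zone name.
; Helpers step back to a linked view, turn in 90-degree steps and normalize mouse position.
; HUD creation and interactable hover tracing are present but disconnected.
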(event `self.ReceiveBeginPlay`
  (bind _returnvalue (`GameplayStatics.GetPlayerController` 0))
  (`WidgetBlueprintLibrary.SetInputMode_GameAndUIEx` _returnvalue null "DoNotLock" false)
  (set `PlayerController.bShowMouseCursor` true _returnvalue)
  (bind _returnvalue_2 (`|CreateWidget` "/Game/Game/UI/WBP_PerformanceBar.WBP_PerformanceBar_C"))
  (`UserWidget.AddToViewport` _returnvalue_2 0))

(event `self.ReceiveTick`
  (params (DeltaSeconds :type "Float (single-precision)")))

(event `Travel To`
  (params (POV :type "PointOfView Object Reference"))
  (set `self.Destination Point of View` POV)
  (`self.Fade Out` (`.HUD` (`self.HUD`)) false)
  (`KismetSystemLibrary.Delay` 0.8)
  (`self.Set Point of View` (`self.Destination Point of View`))
  (set `self.Destination Point of View` null)
  (`self.Fade In` (`.HUD` (`self.HUD`)) false))

(fn `Get Normalized Mouse Position`
  (returns (X :type "Float (double-precision)") (Y :type "Float (double-precision)"))
  (bind (_locationx _locationy) (`PlayerController.GetMousePosition` (`GameplayStatics.GetPlayerController` 0)))
  (bind (_returnvalue_x _returnvalue_y) (`KismetMathLibrary.BreakVector2D` (* (- (/ (`KismetMathLibrary.MakeVector2D` _locationx _locationy) (`WidgetLayoutLibrary.GetViewportSize`)) (0.5 0.5)) (2.0 -2.0))))
  (return _returnvalue_x _returnvalue_y))

(fn `Go Back`
  (returns (`Can go back further` :type Boolean))
  (`self.Travel To` (`PointOfView.Back` (`self.PointOfView`)))
  (return (`KismetSystemLibrary.IsValid` (`PointOfView.Back` (`self.Destination Point of View`)))))

(fn `Look Left`
  (`Pawn.AddControllerYawInput` (`GameplayStatics.GetPlayerPawn` 0) -90.0))

(fn `Look Right`
  (`Pawn.AddControllerYawInput` (`GameplayStatics.GetPlayerPawn` 0) 90.0))

(fn `Set Point of View`
  (params (Actor :type "PointOfView Object Reference"))
  (bind (_hud _hud_2) (`self.HUD`))
  (bind _output_get (set `self.PointOfView` Actor))
  (`self.K2_SetActorLocation` (`GameplayStatics.GetPlayerPawn` 0) (`PointOfView.GetEyeLocation` _output_get) false true)
  (`/Engine/EditorBlueprintResources/StandardMacros.IsValid` _hud_2
    (:`Is Valid`
      (`self.Set Zone Name` _hud_2 (`PointOfView.MapText` (`self.PointOfView`))))))

(fn `UserConstructionScript`)