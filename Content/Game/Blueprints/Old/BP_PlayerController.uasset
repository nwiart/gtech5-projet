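; Player controller for point-and-click interaction, using hovered and clicked actor references stored on BP_Gamemode.
; Holding the left mouse button grabs the hovered actor, which Tick rotates by mouse delta.
; Releasing clears the grab, then either travels through a hovered simple doorway to the first BP_PointOfView found, or teleports a hovered inspect object in front of the current eye location.
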(event `self.ReceiveBeginPlay`
  (`self.SetDeprecatedInputYawScale` 1.0))

(event `self.ReceiveTick`
  (params (DeltaSeconds :type "Float (single-precision)"))
  (bind (_deltax _deltay) (`self.GetInputMouseDelta`))
  (bind _asbp_gamemode (cast `/Game/Game/Blueprints/Old/BP_Gamemode` (`GameplayStatics.GetGameMode`)))
  (bind _clicked_interactible_actor (`/Game/Game/Blueprints/Old/BP_Gamemode.Clicked Interactible Actor` _asbp_gamemode))
  (`/Engine/EditorBlueprintResources/StandardMacros.IsValid` _clicked_interactible_actor
    (:`Is Valid`
      (`self.K2_AddActorWorldRotation` _clicked_interactible_actor (`KismetMathLibrary.MakeRotator` 0.0 (* _deltay -4.0) (* _deltax -4.0)) false true))))

(event `Key|LeftMouseButton`
  (params (Key :type "Key Structure"))
  (bind _returnvalue (`GameplayStatics.GetGameMode`))
  (:`Pressed`
    (bind _asbp_gamemode (cast `/Game/Game/Blueprints/Old/BP_Gamemode` _returnvalue))
    (set `/Game/Game/Blueprints/Old/BP_Gamemode.Clicked Interactible Actor` (`/Game/Game/Blueprints/Old/BP_Gamemode.Hovered Interactible Actor` _asbp_gamemode) _asbp_gamemode))
  (:`Released`
    (bind _asbp_gamemode_2 (cast `/Game/Game/Blueprints/Old/BP_Gamemode` _returnvalue))
    (set `/Game/Game/Blueprints/Old/BP_Gamemode.Clicked Interactible Actor` null _asbp_gamemode_2)
    (bind _hovered_interactible_actor (`/Game/Game/Blueprints/Old/BP_Gamemode.Hovered Interactible Actor` _asbp_gamemode_2))
    (cast `/Game/Game/Blueprints/Interactibles/BP_SimpleDoorway` _hovered_interactible_actor
      (:`then`
        (bind _outactors (`GameplayStatics.GetAllActorsOfClass` "/Game/Game/Blueprints/Old/BP_PointOfView.BP_PointOfView_C"))
        (`/Game/Game/Blueprints/Old/BP_Gamemode.Travel To` _asbp_gamemode_2 (`|GetArrayItem` _outactors)))
      (:`CastFailed`
        (bind _asbp_simple_inspect (cast `/Game/Game/Blueprints/Interactibles/BP_SimpleInspect` _hovered_interactible_actor))
        (`self.K2_SetActorLocation` _asbp_simple_inspect (+ (`PointOfView.GetEyeLocation` (`/Game/Game/Blueprints/Old/BP_Gamemode.PointOfView` _asbp_gamemode_2)) (* (`self.GetActorForwardVector` (`GameplayStatics.GetPlayerPawn` 0)) 200.0)) false true)))))

(fn `UserConstructionScript`)