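; Map trigger actor that moves the player between height levels by linking to a paired destination switcher.
; When the player hits it, it asks the chapter manager from the VN chapter subsystem to travel from itself to that destination.
; The construction script stretches the trigger box and plane mesh to match a configurable width in tiles.
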(event `self.OnPlayerHit`
  (`VNChapterManager.TravelOnHeightSwitcher` (`VNChapterSubsystem.GetChapterManager` (subsystem `VNChapterSubsystem`)) self (`self.Destination Switcher`)))

(fn `UserConstructionScript`
  (`BoxComponent.SetBoxExtent` (`self.Box`) (`KismetMathLibrary.MakeVector` (* (`self.Width in Tiles`) 50.0) 50.0 50.0) true)
  (`SceneComponent.SetRelativeScale3D` (`self.Plane1`) (`KismetMathLibrary.MakeVector` (`KismetMathLibrary.Conv_IntToDouble` (`self.Width in Tiles`)) 1.0 1.0)))