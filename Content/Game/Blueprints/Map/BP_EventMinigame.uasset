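; BP_EventMinigame is a one-shot map event with a bobbing icon and particles that launches a minigame when the player hits it.
; A construction-time GUID keys its save data, which is marked triggered on hit as collision is disabled.
; On BeginPlay, a triggered event destroys itself unless it was the last minigame, in which case it centers the isometric camera on its tile and plays a scale-based disappearance.
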(event `self.ReceiveBeginPlay`
  (bind _returnvalue (`VNSaveSubsystem.GetEventData` (subsystem `VNSaveSubsystem`) (`self.Guid`)))
  (if (`.bTriggered` (break `TableEvents` _returnvalue))
    (if (== (`VNChapterSubsystem.LastMinigameGuid` (subsystem `VNChapterSubsystem`)) (`self.Guid`))
      ; Make sure it can't be hit again
      (`PrimitiveComponent.SetCollisionEnabled` (`self.Box Collision`) "NoCollision")
      ; Position camera on completed minigame
      (bind _aspawn_isometric (cast `PawnIsometric` (`GameplayStatics.GetPlayerPawn` 0)))
      (`PawnIsometric.SetViewCenteredOnTile` _aspawn_isometric (`self.GetTilePosition`))
      ; Animate disappearance
      (bind (_direction _opacity) (`Timeline|Timeline`)
        (:`Update`
          (`SceneComponent.SetRelativeScale3D` (`self.Icon`) (`KismetMathLibrary.MakeVector` _opacity _opacity _opacity))
          (`SceneComponent.SetRelativeScale3D` (`self.PlaneShadow`) (`KismetMathLibrary.MakeVector` _opacity _opacity _opacity)))
        (:`Finished`
          (`ActorComponent.Activate` (`self.ParticleSystem`) false)))
      (else
        (`self.K2_DestroyActor`)))))

(event `self.ReceiveTick`
  (params (DeltaSeconds :type "Float (single-precision)"))
  (bind _returnvalue (`KismetMathLibrary.MakeVector` 0.0 -1.0 (`KismetMathLibrary.MapRangeClamped` (`KismetMathLibrary.Sin` (* (`self.GetGameTimeSinceCreation`) 1.0)) -1.0 1.0 40.0 60.0)))
  (`SceneComponent.K2_SetRelativeLocation` (`self.Icon`) _returnvalue false true)
  (`SceneComponent.K2_SetRelativeLocation` (`self.ParticleSystem`) _returnvalue false true))

(event `self.OnPlayerHit`
  (`VNSaveSubsystem.SetEventData` (subsystem `VNSaveSubsystem`) (`self.Guid`) (make `TableEvents` true))
  ; Make sure it can't be hit again
  (`PrimitiveComponent.SetCollisionEnabled` (`self.Box Collision`) "NoCollision")
  (`VNChapterSubsystem.TriggerMinigame` (subsystem `VNChapterSubsystem`) (`self.Minigame Data`) (`self.Guid`)))

(fn `UserConstructionScript`
  (if (not (`KismetGuidLibrary.IsValid_Guid` (`self.Guid`)))
    (set `self.Guid` (`KismetGuidLibrary.NewGuid`))))