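; BP_PictureFrame is a map actor that animates a picture frame floating along the vertical axis.
; On BeginPlay it stores the root's relative location and sets its Timeline to a random time, so separate instances move out of phase.
; Each Timeline update uses the float track to interpolate the root between that start location and a point a short distance above it.
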(event `self.ReceiveBeginPlay`
  (bind _returnvalue_location (`KismetMathLibrary.BreakTransform` (`SceneComponent.GetRelativeTransform` (`self.DefaultSceneRoot`))))
  (set `self.StartLocation` _returnvalue_location)
  (bind (_direction _floattrack) (`Timeline|Timeline` :`NewTime` (`KismetMathLibrary.RandomFloatInRange` 0.0 4.0) :!via `SetNewTime`)
    (:`Update`
      (`SceneComponent.K2_SetRelativeLocation` (`self.DefaultSceneRoot`) (`KismetMathLibrary.VLerp` (`self.StartLocation`) (+ (`self.StartLocation`) (0.0 0.0 50.0)) _floattrack) false false))))

(fn `UserConstructionScript`)