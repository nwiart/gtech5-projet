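; BP_ObjectiveDialogue is a one-time map pickup with a bobbing icon that runs a dialogue when the player hits it.
; A GUID assigned in construction keys its triggered state in VNSaveSubsystem, so it destroys itself on later loads.
; On hit it saves, disables collision and runs any assigned dialogue through BP_GamemodeNoah.
; When dialogue ends, or immediately without one, a timeline scales icon and shadow, then activates particles.
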(event `self.ReceiveBeginPlay`
  (bind _returnvalue (`VNSaveSubsystem.GetEventData` (subsystem `VNSaveSubsystem`) (`self.Guid`)))
  (if (`.bTriggered` (break `TableEvents` _returnvalue))
    (`self.K2_DestroyActor`)))

(event `self.ReceiveTick`
  (params (DeltaSeconds :type "Float (single-precision)"))
  (bind _returnvalue (`KismetMathLibrary.MakeVector` 0.0 -1.0 (`KismetMathLibrary.MapRangeClamped` (`KismetMathLibrary.Sin` (* (`self.GetGameTimeSinceCreation`) 1.0)) -1.0 1.0 40.0 60.0)))
  (`SceneComponent.K2_SetRelativeLocation` (`self.Icon`) _returnvalue false true)
  (`SceneComponent.K2_SetRelativeLocation` (`self.ParticleSystem`) _returnvalue false true))

(event `self.OnPlayerHit`
  (bind _dialogue_to_play (`self.Dialogue To Play`))
  ; Save "triggered" state
  (bind _output_get (set `self.Data` (make `TableEvents` true)))
  (`VNSaveSubsystem.SetEventData` (subsystem `VNSaveSubsystem`) (`self.Guid`) _output_get)
  ; Make sure it can't be hit again
  (`PrimitiveComponent.SetCollisionEnabled` (`self.Box Collision`) "NoCollision")
  (`/Engine/EditorBlueprintResources/StandardMacros.IsValid` _dialogue_to_play
    (:`Is Valid`
      (bind _asbp_gamemode_noah (cast `/Game/Game/Blueprints/Map/Gameplay/BP_GamemodeNoah` (`GameplayStatics.GetGameMode`)))
      (`/Game/Game/Blueprints/Map/Gameplay/BP_GamemodeNoah.Run Dialogue` _asbp_gamemode_noah _dialogue_to_play)
      (add `/Game/Game/Blueprints/Map/Gameplay/BP_GamemodeNoah.On Dialogue Sequence End` _asbp_gamemode_noah (delegate `CustomEvent`)))
    (:`Is Not Valid`
      ; Animate disappearance
      (bind (_direction _opacity) (`Timeline|Timeline` :!label _label)
        (:`Update`
          (`SceneComponent.SetRelativeScale3D` (`self.Icon`) (`KismetMathLibrary.MakeVector` _opacity _opacity _opacity))
          (`SceneComponent.SetRelativeScale3D` (`self.PlaneShadow`) (`KismetMathLibrary.MakeVector` _opacity _opacity _opacity)))
        (:`Finished`
          (`ActorComponent.Activate` (`self.ParticleSystem`) false))))))

(event `CustomEvent`
  (params (NewParam :type "DialogueLineSequence Object Reference"))
  (goto _label))

(fn `UserConstructionScript`
  (if (not (`KismetGuidLibrary.IsValid_Guid` (`self.Guid`)))
    (set `self.Guid` (`KismetGuidLibrary.NewGuid`))))