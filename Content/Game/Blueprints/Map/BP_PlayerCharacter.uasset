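; Player character Blueprint with a slot-based inventory and a sprite opacity fade.
; Pressing I picks up the first overlapping BP_InventoryItem into a matching or empty slot, updates WBP_Inventory and destroys the item.
; Separate events decrement slots, spawn a slot's stored class ahead with random sideways offset, and FlipFlop the inventory's visibility and input mode.
; FadeOut and FadeIn play one Timeline forward or backward on a dynamic material.
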(event `self.ReceiveTick`
  (params (DeltaSeconds :type "Float (single-precision)")))

(event `self.ReceiveBeginPlay`
  (bind _inventorywidget (`self.InventoryWidget`))
  (bind _returnvalue (`|CreateWidget` "/Game/Game/UI/InventorySystem/WBP_Inventory.WBP_Inventory_C"))
  (set `self.InventoryWidget` _returnvalue)
  (`UserWidget.AddToViewport` _inventorywidget 0)
  (set `Widget.Visibility` "Hidden" _inventorywidget)
  (`KismetSystemLibrary.PrintString` "aaaaaaaaaaaaaaaaaaaaaaaaaaaaaaaaaaaaaaaaaaaaaaaaaaaaaaaaaaaaaaaaaaaaaaaaaaaaaaaaaaaaaaaaaaa"))

(event `Fade Out`
  (bind _sprite (`self.Sprite`))
  (bind _returnvalue (`PrimitiveComponent.CreateDynamicMaterialInstance` _sprite 0 (`PrimitiveComponent.GetMaterial` _sprite 0) "None"))
  (set `self.Dynamic Material` _returnvalue)
  (bind (_direction _opacity) (`Timeline|Timeline` :!via `PlayFromStart` :!label _label)
    (:`Update`
      (`MaterialInstanceDynamic.SetScalarParameterValue` (`self.Dynamic Material`) "Opacity" _opacity))))

(event `Fade In`
  (bind _sprite (`self.Sprite`))
  (bind _returnvalue (`PrimitiveComponent.CreateDynamicMaterialInstance` _sprite 0 (`PrimitiveComponent.GetMaterial` _sprite 0) "None"))
  (set `self.Dynamic Material` _returnvalue)
  (goto _label :!via `ReverseFromEnd`))

(event `Key|I`
  (params (Key :type "Key Structure"))
  (:`Pressed`
    (`self.FillSlot`)
    (`KismetSystemLibrary.PrintString` "tesr")))

(event `ChangeInventoryMenuStatus`
  (bind _returnvalue (`GameplayStatics.GetPlayerController` 0))
  (bind _inventorywidget (`self.InventoryWidget`))
  (`/Engine/EditorBlueprintResources/StandardMacros.FlipFlop`
    (:`A`
      (set `Widget.Visibility` "Visible" _inventorywidget)
      (`WidgetBlueprintLibrary.SetInputMode_GameAndUIEx` _returnvalue null)
      (set `PlayerController.bShowMouseCursor` true _returnvalue))
    (:`B`
      (set `Widget.Visibility` "Hidden" _inventorywidget)
      (`WidgetBlueprintLibrary.SetInputMode_GameOnly` (`GameplayStatics.GetPlayerController` 0)))))

(event `FillSlot`
  (bind _inventoryslots (`self.InventorySlots`))
  (bind _itemdetails_name (break `/Game/Game/Blueprints/InventorySystem/ItemDetails` (`/Game/Game/Blueprints/InventorySystem/BP_InventoryItem.ItemDetails` (`self.TargetItem`))))
  (bind (_itemdetails_name_2 _itemdetails_image) (break `/Game/Game/Blueprints/InventorySystem/ItemDetails` (`/Game/Game/Blueprints/InventorySystem/BP_InventoryItem.ItemDetails` (`self.TargetItem`))))
  (`KismetSystemLibrary.PrintString` "Item picked")
  (bind _output_get (set `self.TargetItem` (`|GetArrayItem` (`self.GetOverlappingActors` "/Game/Game/Blueprints/InventorySystem/BP_InventoryItem.BP_InventoryItem_C"))))
  (`/Engine/EditorBlueprintResources/StandardMacros.IsValid` _output_get
    (:`Is Valid`
      (for (_array_element _array_index) _inventoryslots
        (bind _itemdetails_name_3 (break `/Game/Game/Blueprints/InventorySystem/ItemDetails` (`/Game/Game/Blueprints/InventorySystem/BP_InventoryItem.ItemDetails` _output_get)))
        (if (or (`KismetStringLibrary.EqualEqual_StrStr` (break `/Game/Game/Blueprints/InventorySystem/ItemSlotData` _array_element) _itemdetails_name_3) (`.IsEmpty_5_F5E0D4214DDB2B39B01DEA9FAFA7679F` (break `/Game/Game/Blueprints/InventorySystem/ItemSlotData` _array_element)))
          (break)))
      (bind _output (`|GetArrayItem` _inventoryslots _array_index))
      (bind (_name _quantity _isempty) (break `/Game/Game/Blueprints/InventorySystem/ItemSlotData` _output))
      (if _isempty
        (bind _slot (`/Game/Game/UI/InventorySystem/WBP_Inventory.GetSlotAtIndex` (`self.InventoryWidget`) _array_index))
        (bind _itemimage (`/Game/Game/UI/InventorySystem/WBP_InventoryButton.ItemImage` _slot))
        (set `Widget.Visibility` "SelfHitTestInvisible" _itemimage)
        (set `Widget.Visibility` "SelfHitTestInvisible" (`/Game/Game/UI/InventorySystem/WBP_InventoryButton.Border_207` _slot))
        (set `/Game/Game/UI/InventorySystem/WBP_InventoryButton.SlotNb` _array_index _slot)
        (bind _structout (setmembers `/Game/Game/Blueprints/InventorySystem/ItemSlotData` :`StructRef` _output :`Name` _itemdetails_name_2 :`Quantity` (+ _quantity 1) :`IsEmpty` false :`Image` _itemdetails_image :`Class` (`GameplayStatics.GetObjectClass` (`self.TargetItem`)) :!label _label_2))
        (`Image.SetBrushFromTexture` _itemimage (`.Image_12_AC584F87482D575AA9A407870B36DDC5` (break `/Game/Game/Blueprints/InventorySystem/ItemSlotData` _structout)) false)
        (set `TextBlock.Text` (`KismetTextLibrary.Conv_IntToText` (`.Quantity_11_0FDBB64F4EABCFEAE6695EBF8BFD075F` (break `/Game/Game/Blueprints/InventorySystem/ItemSlotData` _structout))) (`/Game/Game/UI/InventorySystem/WBP_InventoryButton.Quantity` _slot))
        (`self.K2_DestroyActor` null)
        (`self.K2_DestroyActor` (`self.TargetItem`))
        (elif (`KismetStringLibrary.EqualEqual_StrStr` _name _itemdetails_name)
          (goto _label_2)
          (else
            (`KismetSystemLibrary.PrintString` "Full inventory")))))))

(event `UnFillSlot`
  (params (`Slot Nb` :type Integer))
  (bind _slot (`/Game/Game/UI/InventorySystem/WBP_Inventory.GetSlotAtIndex` (`self.InventoryWidget`) `Slot Nb`))
  (bind _output (`|GetArrayItem` (`self.InventorySlots`) `Slot Nb`))
  (bind (_name _quantity _isempty _image) (break `/Game/Game/Blueprints/InventorySystem/ItemSlotData` _output))
  (bind _itemimage (`/Game/Game/UI/InventorySystem/WBP_InventoryButton.ItemImage` _slot))
  (bind _returnvalue (- _quantity 1))
  (bind _returnvalue_2 (> _returnvalue 0))
  (bind _structout (setmembers `/Game/Game/Blueprints/InventorySystem/ItemSlotData` :`StructRef` _output :`Name` (select `bool` _returnvalue_2 :`true` _name) :`Quantity` (select `bool` _returnvalue_2 :`true` _returnvalue) :`IsEmpty` (select `bool` _returnvalue_2 :`false` true) :`Image` (select `bool` _returnvalue_2 :`true` _image)))
  (if (`.IsEmpty_5_F5E0D4214DDB2B39B01DEA9FAFA7679F` (break `/Game/Game/Blueprints/InventorySystem/ItemSlotData` _structout))
    (set `Widget.Visibility` "Hidden" (`/Game/Game/UI/InventorySystem/WBP_InventoryButton.Border_207` _slot))
    (set `Widget.Visibility` "Hidden" _itemimage)
    (`Image.SetBrushFromTexture` _itemimage null false))
  (`TextBlock.SetText` (`/Game/Game/UI/InventorySystem/WBP_InventoryButton.Quantity` _slot) (`KismetTextLibrary.Conv_IntToText` (`.Quantity_11_0FDBB64F4EABCFEAE6695EBF8BFD075F` (break `/Game/Game/Blueprints/InventorySystem/ItemSlotData` _structout)))))

(event `DropItem`
  (params (`Slot Nb` :type Integer))
  (`|SpawnActorFromClass` (`.Class_14_570EE012406168F393A37CB252683758` (break `/Game/Game/Blueprints/InventorySystem/ItemSlotData` (`|GetArrayItem` (`self.InventorySlots`) `Slot Nb`))) (`KismetMathLibrary.MakeTransform` (+ (`self.K2_GetActorLocation`) (* (`self.GetActorForwardVector`) 50) (* (`self.GetActorRightVector`) (`KismetMathLibrary.RandomFloatInRange` -35.0 35.0)))) "Undefined" "MultiplyWithRoot" null null))

(fn `UserConstructionScript`)