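; BP_ChapterManager runs a visual novel chapter's UI flow: HUD, dialogue and minigame launches.
; It creates the HUD and dialogue widgets on BeginPlay, then shows the HUD when enabled.
; Dialogue fades out the HUD and disables the pawn's cursor, restoring both when it ends.
; Minigames switch to UI-only input, hide the HUD, show a timed name announcement, then async-load their level behind a loading screen.
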(event `self.ReceiveBeginPlay`
  (bind _returnvalue (`|CreateWidget` "/Game/Game/UI/GameHUB/WBP_HUD.WBP_HUD_C"))
  (set `self.HUD` _returnvalue)
  (bind _returnvalue_2 (`|CreateWidget` "/Game/Game/UI/Dialogue/WB_Dialogue.WB_Dialogue_C"))
  (bind _output_get (set `self.Dialogue UI` _returnvalue_2))
  (add `/Game/Game/UI/Dialogue/WB_Dialogue.On Dialogue Ended` _output_get (delegate `On Dialogue End`)))

(event `self.Enable`
  (`parent.Enable`)
  (`UserWidget.AddToViewport` (`self.HUD`) 0))

(event `self.ReceiveEndPlay`
  (params (EndPlayReason :type "EEndPlayReason Enum" :default "Destroyed"))
  (`Widget.RemoveFromParent` (`self.HUD`))
  (`Widget.RemoveFromParent` (`self.Dialogue UI`)))

(event `Run Dialogue`
  (params (`Dialogue Line Sequence` :type "DialogueLineSequence Object Reference"))
  (`PawnIsometric.SetCursorActive` (`VNChapterSubsystem.GetPawn` (subsystem `VNChapterSubsystem`)) false)
  (`/Game/Game/UI/GameHUB/WBP_HUD.Fade Out` (`self.HUD`) false)
  (`KismetSystemLibrary.Delay` 0.6)
  (`UserWidget.AddToViewport` (`self.Dialogue UI`) 0)
  (`/Game/Game/UI/Dialogue/WB_Dialogue.Run Dialogue` (`self.Dialogue UI`) `Dialogue Line Sequence`))

(event `On Dialogue End`
  (`/Game/Game/UI/GameHUB/WBP_HUD.Fade In` (`self.HUD`) false)
  (`KismetSystemLibrary.Delay` 0.6)
  (`PawnIsometric.SetCursorActive` (`VNChapterSubsystem.GetPawn` (subsystem `VNChapterSubsystem`)) true))

(event `self.TriggerMinigame`
  (params (Minigame :type "MinigameData Structure (by ref)"))
  (bind (_name _description _level) (break `MinigameData` Minigame))
  (`parent.TriggerMinigame` Minigame)
  (`WidgetBlueprintLibrary.SetInputMode_UIOnlyEx` (`GameplayStatics.GetPlayerController` 0) null)
  (`KismetSystemLibrary.Delay` 1.0)
  (`Widget.SetVisibility` (`self.HUD`) "Hidden")
  (bind _returnvalue (`|CreateWidget` "/Game/Game/UI/Minigame/WBP_MinigameAnnounce.WBP_MinigameAnnounce_C"))
  (`UserWidget.AddToViewport` _returnvalue 0)
  (set `TextBlock.Text` (`KismetTextLibrary.Conv_NameToText` _name) (`/Game/Game/UI/Minigame/WBP_MinigameAnnounce.TextGameName` _returnvalue))
  (`KismetSystemLibrary.Delay` 3.0)
  (cast `VNGameInstance` (`GameplayStatics.GetGameInstance`))
  (`SceneTransitionSubsystem.LoadLevelAsync` (subsystem `SceneTransitionSubsystem`) _level "/Game/Game/UI/LoadingSystem/WBP_LoadingScreen.WBP_LoadingScreen_C")
  (`KismetSystemLibrary.Delay` 1.0)
  (`Widget.RemoveFromParent` _returnvalue))

(fn `UserConstructionScript`
  (`parent.UserConstructionScript`))