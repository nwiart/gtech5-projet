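; Global player controller that registers itself with BP_GameInstance and provides hold-to-quit for the game.
; On level load it re-registers, creates a hidden WB_QuitGame widget stored on the game instance, and sets Game-and-UI input mode.
; Holding QuitHold shows the widget while Tick accumulates hold time and updates its text, quitting at MaxHoldTime.
; Releasing early resets the timer and hides the widget.
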(event `self.ReceiveBeginPlay`
  (bind _asbp_game_instance (cast `/Game/Game/Blueprints/BP_GameInstance` (`GameplayStatics.GetGameInstance`)))
  (bind _output_get (set `self.BP Game Instance` _asbp_game_instance))
  (`/Game/Game/Blueprints/BP_GameInstance.RegisterController` _output_get)
  (`WidgetBlueprintLibrary.SetFocusToGameViewport`)
  (add `self.OnLevelLoaded` (delegate `OnLevelLoaded_Event`)))

(event `OnLevelLoaded_Event`
  (bind _bp_game_instance (`self.BP Game Instance`))
  (bind _quitwidget (`/Game/Game/Blueprints/BP_GameInstance.QuitWidget` _bp_game_instance))
  (`|ExecutionSequence`
    (:`then_0`
      (bind _returnvalue (`|CreateWidget` "/Game/Game/UI/Menu/WB_QuitGame.WB_QuitGame_C"))
      (set `/Game/Game/Blueprints/BP_GameInstance.QuitWidget` _returnvalue _bp_game_instance)
      (`Widget.SetVisibility` _returnvalue "Hidden"))
    (:`then_1`
      (`/Game/Game/Blueprints/BP_GameInstance.RegisterController` _bp_game_instance)
      (`UserWidget.AddToViewport` _quitwidget 0)
      (`WidgetBlueprintLibrary.SetInputMode_GameAndUIEx` self _quitwidget "DoNotLock" false)
      (`WidgetBlueprintLibrary.SetFocusToGameViewport`))))

(event `InputAction|QuitHold` :paused true
  (params (Key :type "Key Structure"))
  (bind _quitwidget (`/Game/Game/Blueprints/BP_GameInstance.QuitWidget` (`self.BP Game Instance`)))
  (:`Pressed`
    (`UserWidget.AddToViewport` (`/Game/Game/Blueprints/BP_GameInstance.QuitWidget` (`self.BP Game Instance`)) 0)
    (set `self.IsHoldingQuit` true)
    (set `self.HoldTime` 0.0)
    (set `Widget.Visibility` "Visible" _quitwidget))
  (:`Released`
    (set `self.IsHoldingQuit` false)
    (set `self.HoldTime` 0.0)
    (set `Widget.Visibility` "Hidden" _quitwidget)))

(event `self.ReceiveTick`
  (params (DeltaSeconds :type "Float (single-precision)"))
  (if (`self.IsHoldingQuit`)
    (bind _output_get (set `self.HoldTime` (+ (`self.HoldTime`) DeltaSeconds)))
    (`/Game/Game/UI/Menu/WB_QuitGame.UpdateQuitText` (`/Game/Game/Blueprints/BP_GameInstance.QuitWidget` (`self.BP Game Instance`)) _output_get)
    (if (>= _output_get (`self.MaxHoldTime`))
      (`KismetSystemLibrary.QuitGame` null "Quit"))))

(fn `UserConstructionScript`)