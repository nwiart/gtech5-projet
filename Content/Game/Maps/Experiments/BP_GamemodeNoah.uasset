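; Experimental game mode that hosts a test of the dialogue UI.
; BeginPlay creates the WB_Dialogue widget up front.
; RunTestDialogue fades out the HUD, sets the left speaker from the CurrentDialogueLine class defaults, shows the widget, then starts dialogue on an object constructed from that class.
; EndDialogue fades the dialogue out and the HUD back in, with fixed delays pacing both transitions.
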(event `self.ReceiveBeginPlay`
  (`parent.ReceiveBeginPlay`)
  (bind _returnvalue (`|CreateWidget` "/Game/Game/UI/WB_Dialogue.WB_Dialogue_C"))
  (set `self.Dialogue UI` _returnvalue))

(event `Run Test Dialogue`
  (bind _dialogue_ui (`self.Dialogue UI`))
  (`/Game/Game/UI/WB_HUD.Fade Out` (`self.HUD`) false)
  (`KismetSystemLibrary.Delay` 0.6)
  (`/Game/Game/UI/WB_Dialogue.Set Characters` (`self.Dialogue UI`) (`.Character` (break `DialogueLine` (`|GetArrayItem` (defaults `Object` (`self.Current Dialogue Line`))))) null)
  (`UserWidget.AddToViewport` _dialogue_ui 0)
  (`/Game/Game/UI/WB_Dialogue.Fade In` _dialogue_ui)
  (`KismetSystemLibrary.Delay` 0.6)
  (bind _returnvalue (`|GenericCreateObject` (`self.Current Dialogue Line`)))
  (`/Game/Game/UI/WB_Dialogue.Begin Dialogue` _dialogue_ui _returnvalue))

(event `End Dialogue`
  (`/Game/Game/UI/WB_Dialogue.Fade Out` (`self.Dialogue UI`))
  (`KismetSystemLibrary.Delay` 0.6)
  (`/Game/Game/UI/WB_HUD.Fade In` (`self.HUD`) false)
  (`KismetSystemLibrary.Delay` 0.6))

(fn `UserConstructionScript`
  (`parent.UserConstructionScript`))