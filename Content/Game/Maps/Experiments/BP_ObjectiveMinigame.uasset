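; BP_ObjectiveMinigame is an objective marker that launches a minigame when its player-hit event fires.
; Each Tick, a sine of game time since creation bobs the Icon and ParticleSystem components vertically in sync.
; OnPlayerHit casts the game mode to BP_GamemodeNoah and calls TriggerMinigame with the actor's minigame level and name.
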(event `self.ReceiveTick`
  (params (DeltaSeconds :type "Float (single-precision)"))
  (bind _returnvalue (`KismetMathLibrary.MakeVector` 0.0 -1.0 (`KismetMathLibrary.MapRangeClamped` (`KismetMathLibrary.Sin` (* (`self.GetGameTimeSinceCreation`) 1.0)) -1.0 1.0 40.0 60.0)))
  (`SceneComponent.K2_SetRelativeLocation` (`self.Icon`) _returnvalue false true)
  (`SceneComponent.K2_SetRelativeLocation` (`self.ParticleSystem`) _returnvalue false true))

(event `self.OnPlayerHit`
  (bind _asbp_gamemode_noah (cast `/Game/Game/Maps/Experiments/Gameplay/BP_GamemodeNoah` (`GameplayStatics.GetGameMode`)))
  (`/Game/Game/Maps/Experiments/Gameplay/BP_GamemodeNoah.Trigger Minigame` _asbp_gamemode_noah (`self.Minigame Level`) (`self.Minigame Name`)))

(fn `UserConstructionScript`)