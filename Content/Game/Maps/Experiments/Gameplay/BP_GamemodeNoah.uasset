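; Experimental game mode that owns the HUD and dialogue UI and handles transitions into minigames.
; On BeginPlay it shows the cursor and creates both widgets, adding only the HUD to the viewport.
; Dialogue events fade between HUD and dialogue widget using timed delays, then fire an end-of-sequence callback with the current line.
; Triggering a minigame switches to UI-only input, replaces the HUD with a named announcement, then opens the given level.
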(event `self.ReceiveBeginPlay`
  (bind _returnvalue (`GameplayStatics.GetPlayerController` 0))
  (`WidgetBlueprintLibrary.SetInputMode_GameAndUIEx` _returnvalue null "DoNotLock" false)
  (set `PlayerController.bShowMouseCursor` true _returnvalue)
  (bind _returnvalue_2 (`|CreateWidget` "/Game/Game/UI/WB_HUD.WB_HUD_C"))
  (bind _output_get (set `self.HUD` _returnvalue_2))
  (`UserWidget.AddToViewport` _returnvalue_2 0)
  (`UserWidget.AddToViewport` _output_get 0)
  (bind _returnvalue_3 (`|CreateWidget` "/Game/Game/UI/WB_Dialogue.WB_Dialogue_C"))
  (set `self.Dialogue UI` _returnvalue_3))

(event `Run Test Dialogue`
  (bind _dialogue_ui (`self.Dialogue UI`))
  (`/Game/Game/UI/WB_HUD.Fade Out` (`self.HUD`) false :!label _label)
  (`KismetSystemLibrary.Delay` 0.6)
  (`/Game/Game/UI/WB_Dialogue.Set Characters` (`self.Dialogue UI`) (`self.Current Dialogue Line`))
  (`UserWidget.AddToViewport` _dialogue_ui 0)
  (`/Game/Game/UI/WB_Dialogue.Fade In` _dialogue_ui)
  (`KismetSystemLibrary.Delay` 0.6)
  (`/Game/Game/UI/WB_Dialogue.Begin Dialogue` _dialogue_ui (`self.Current Dialogue Line`)))

(event `Run Dialogue`
  (params (NewParam :type "DialogueLineSequence Object Reference"))
  (set `self.Current Dialogue Line` NewParam)
  (goto _label))

(event `End Dialogue`
  (`/Game/Game/UI/WB_Dialogue.Fade Out` (`self.Dialogue UI`))
  (`KismetSystemLibrary.Delay` 0.6)
  (`self.On Dialogue Sequence End` (`self.Current Dialogue Line`))
  (`/Game/Game/UI/WB_HUD.Fade In` (`self.HUD`) false)
  (`KismetSystemLibrary.Delay` 0.6))

(event `Trigger Minigame`
  (params (Level :type "SoftWorldReference Structure") (Name :type Name))
  (`KismetSystemLibrary.Delay` 1.0)
  (`WidgetBlueprintLibrary.SetInputMode_UIOnlyEx` (`GameplayStatics.GetPlayerController` 0) null)
  (`Widget.RemoveFromParent` (`self.HUD`))
  (bind _returnvalue (`|CreateWidget` "/Game/Game/UI/WB_MinigameAnnounce.WB_MinigameAnnounce_C"))
  (`UserWidget.AddToViewport` _returnvalue 0)
  (set `TextBlock.Text` (`KismetTextLibrary.Conv_NameToText` Name) (`/Game/Game/UI/WB_MinigameAnnounce.TextGameName` _returnvalue))
  (`KismetSystemLibrary.Delay` 3.0)
  (`/Game/Game/UI/WB_MinigameAnnounce.Fade Out` _returnvalue)
  (`KismetSystemLibrary.Delay` 1.0)
  (`GameplayStatics.OpenLevelBySoftObjectPtr` (`.WorldAsset` (break `SoftWorldReference` Level))))

(fn `UserConstructionScript`
  (`parent.UserConstructionScript`))