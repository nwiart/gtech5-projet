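; BP_EndGame is a level actor that ends the current chapter when its OnPlayerHit event fires.
; It fetches the chapter statistics for the current level name from BP_SaveGame via VNSaveSubsystem's SaveManager and displays them in a WBP_EndGameScreen widget.
; It hands its NextScene value to that widget, pauses the game and saves through the SaveManager.
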(event `self.OnPlayerHit`
  (bind _savemanager (`VNSaveSubsystem.SaveManager` (subsystem `VNSaveSubsystem`)))
  (bind _asbp_save_game (cast `/Game/Game/Blueprints/BP_SaveGame` (`VNSaveManager.SaveGame` _savemanager)))
  (bind _returnvalue (`GameplayStatics.GetCurrentLevelName` true))
  (`self.ShowEndGameStats` (`/Game/Game/Blueprints/BP_SaveGame.Get Chapter Statistics` _asbp_save_game (`KismetStringLibrary.Conv_StringToName` _returnvalue)))
  (`GameplayStatics.SetGamePaused` true)
  (`VNSaveManager.Save` _savemanager))

(fn `ShowEndGameStats`
  (params (`Chapter Stats` :type "/Game/Game/Blueprints/EndGame/ST_EndGameStat Structure"))
  (bind _returnvalue (`|CreateWidget` "/Game/Game/UI/EndGame/WBP_EndGameScreen.WBP_EndGameScreen_C"))
  (`UserWidget.AddToViewport` _returnvalue 0)
  (`/Game/Game/UI/EndGame/WBP_EndGameScreen.BuildEndGameStats` _returnvalue `Chapter Stats`)
  (set `/Game/Game/UI/EndGame/WBP_EndGameScreen.NextScene` (`self.NextScene`) _returnvalue))

(fn `UserConstructionScript`)