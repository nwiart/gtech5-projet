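; BP_EndGame is an actor that ends the game with a stats screen when its OnPlayerHit event fires.
; The event reads GameStats from BP_GamemodeNoah, shows the screen, then pauses the game.
; ShowEndGameStats creates a WBP_EndGameScreen, adds it to the viewport, builds it from those stats and passes on the actor's NextScene.
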(event `self.OnPlayerHit`
  (bind _asbp_gamemode_noah (cast `/Game/Game/Levels/Experiments/Gameplay/BP_GamemodeNoah` (`GameplayStatics.GetGameMode`)))
  (`self.ShowEndGameStats` (`/Game/Game/Levels/Experiments/Gameplay/BP_GamemodeNoah.GameStats` _asbp_gamemode_noah))
  (`GameplayStatics.SetGamePaused` true))

(fn `ShowEndGameStats`
  (params (NewParam :type "Array of /Game/Game/Blueprints/EndGame/ST_EndGameStat Structure"))
  (bind _returnvalue (`|CreateWidget` "/Game/Game/UI/EndGame/WBP_EndGameScreen.WBP_EndGameScreen_C"))
  (`UserWidget.AddToViewport` _returnvalue 0)
  (`/Game/Game/UI/EndGame/WBP_EndGameScreen.BuildEndGameStats` _returnvalue NewParam)
  (set `/Game/Game/UI/EndGame/WBP_EndGameScreen.NextScene` (`self.NextScene`) _returnvalue))

(fn `UserConstructionScript`)